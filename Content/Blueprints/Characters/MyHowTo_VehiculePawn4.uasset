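; Vehicle pawn Blueprint with a weapon mesh and weapon component, whose only active logic visualizes weapon aiming.
; Each Tick draws a debug sphere at the weapon target position and a green debug line to it from the muzzle.
; The muzzle point comes from rotating the weapon component's muzzle offset by the weapon mesh's world rotation and adding its world location.
; An unused forward-vector projection remains unconnected.
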(event `self.ReceiveTick`
  (params (DeltaSeconds :type "Float (single-precision)"))
  (bind _weapontargetpos (`self.WeaponTargetPos`))
  (bind _weaponmesh (`self.WeaponMesh`))
  (`KismetSystemLibrary.DrawDebugSphere` _weapontargetpos)
  (`KismetSystemLibrary.DrawDebugLine` (+ (`SceneComponent.K2_GetComponentLocation` _weaponmesh) (`KismetMathLibrary.GreaterGreater_VectorRotator` (`WeaponComponent.MuzzleOffset` (`self.WeaponComponent`)) (`SceneComponent.K2_GetComponentRotation` _weaponmesh))) _weapontargetpos (struct :`G` 0.848958 :`B` 0.098487 :`A` 1.0)))

(fn `UserConstructionScript`)