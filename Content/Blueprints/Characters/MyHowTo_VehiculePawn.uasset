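; Vehicle pawn Blueprint that keeps its weapon mesh pointed along the camera's aim direction.
; Each Tick, UpdateWeaponsRotation sets the weapon's world rotation to a look-at rotation toward a distant point along the camera's forward vector.
; The look-at start and target are built from the weapon's and camera's relative locations rather than world locations, combined with the world-space forward vector.
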(event `self.ReceiveTick`
  (params (DeltaSeconds :type "Float (single-precision)"))
  (`self.UpdateWeaponsRotation`))

(fn `GetWeaponNewRotation`
  (params (WeaponLocation :type "Vector Structure"))
  (returns (NewRotation :type "Rotator Structure"))
  (bind _newparam (`self.GetWeaponTargetPosition` self))
  (return (`KismetMathLibrary.FindLookAtRotation` WeaponLocation _newparam)))

(fn `GetWeaponTargetPosition`
  (returns (NewParam :type "Vector Structure"))
  (bind _camera (`self.Camera`))
  (return (+ (* (`SceneComponent.GetForwardVector` _camera) 10000.0) (`SceneComponent.RelativeLocation` _camera))))

(fn `UpdateWeaponsRotation`
  (bind _newrotation (`self.GetWeaponNewRotation` (`SceneComponent.RelativeLocation` (`self.WeaponMesh`))))
  (`SceneComponent.K2_SetWorldRotation` (`self.WeaponMesh`) _newrotation false false))

(fn `UserConstructionScript`)